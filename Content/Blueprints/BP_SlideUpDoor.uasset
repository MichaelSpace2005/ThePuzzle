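; BP_SlideUpDoor is a door that slides to an offset once every linked size checker is activated.
; The construction script gives the DoorMovement component two relative control points, the origin and MoveToPos.
; Tick polls the SizeCheckers array while the door is closed, counting activated entries and resetting at the first inactive one.
; When the count matches the array length, OpenDoor activates the movement and sets DoorIsOpen, which stops further checks.
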(event Custom|OpenDoor
  (Components|Activation|Activate (Variables|Default|GetDoorMovement) false)
  (Variables|Default|SetbDoorIsOpen true))

(event EventTick
  (params (DeltaSeconds :type Float%20%28single-precision%29))
  (if (and (Utilities|Array|IsNotEmpty (Variables|Default|GetSizeCheckers)) (not (Variables|Default|GetbDoorIsOpen)))
    (bind _array_element (Utilities|Array|ForEachLoopwithBreak (Variables|Default|GetSizeCheckers) :!label _label)
      (:LoopBody
        (if (Variables|/Game/Blueprints/SizeCheckers/BP_SizeChecker.BP_SizeChecker_C|GetbIsActivated _array_element)
          (Math|Integer|IncrementInt (Variables|Default|GetNumberOfActCheckers))
          (else
            (Variables|Default|SetNumberOfActCheckers 0)
            (goto _label Break))))
      (:Completed
        (if (== (Variables|Default|GetNumberOfActCheckers) (Utilities|Array|Length (Variables|Default|GetSizeCheckers)))
          (CallFunction|OpenDoor))))))

(fn ConstructionScript
  (Class|InterptoMovementComponent|AddControlPointPosition (Variables|Default|GetDoorMovement) "0, 0, 0" true)
  (Class|InterptoMovementComponent|AddControlPointPosition (Variables|Default|GetDoorMovement) (Variables|Default|GetMoveToPos) true))