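; BP_InteractButton is an interact button triggered by objects that overlap its collision, apparently intended as a base for specific buttons.
; A flag selects whether it responds only to the assigned GrabObj or to any actor tagged GrabbleObject.
; Each mode fires its own event: SpecialObjectActivate is an empty stub and AnyObjectActivate only prints a debug string.
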(event OnComponentBeginOverlap(Collision)
  (params (OverlappedComponent :type Primitive%20Component%20Object%20Reference) (OtherActor :type Actor%20Object%20Reference) (OtherComp :type Primitive%20Component%20Object%20Reference) (OtherBodyIndex :type Integer) (bFromSweep :type Boolean) (SweepResult :type Hit%20Result%20Structure%20%28by%20ref%29))
  (if (Variables|Default|GetbIsUSpecialObj)
    (if (== OtherActor (Variables|Default|GetGrabObj))
      (CallFunction|SpecialObjectActivate))
    (elif (Actor|ActorHasTag OtherActor "GrabbleObject")
      (CallFunction|AnyObjectActivate))))

(event Custom|AnyObjectActivate
  (Development|PrintString "BaseAnyObject" true true "(R=0.126284,G=1.000000,B=0.000000,A=1.000000)"))

(event Custom|SpecialObjectActivate)

(fn ConstructionScript)