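; BP_Scaler is a trigger volume that switches scaling or unscaling on for the object the player is grabbing.
; On begin overlap by an actor tagged "GrabbleObject", ScaleType selects which flag to set; end overlap clears both.
; Flags are written to the cached player character's CurrentGrabbleObj rather than the overlapping actor, leaving the resizing to that object.
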(event OnComponentBeginOverlap(Box)
  (params (OverlappedComponent :type Primitive%20Component%20Object%20Reference) (OtherActor :type Actor%20Object%20Reference) (OtherComp :type Primitive%20Component%20Object%20Reference) (OtherBodyIndex :type Integer) (bFromSweep :type Boolean) (SweepResult :type Hit%20Result%20Structure%20%28by%20ref%29))
  (if (Actor|ActorHasTag OtherActor "GrabbleObject")
    (if (Utilities|Enum|Equal(Enum) (Variables|Default|GetScaleType) "NewEnumerator2")
      (bind _currentgrabbleobj (Variables|/Game/Blueprints/PlayerCharacter/BP_PlayerCharacter.BP_PlayerCharacter_C|GetCurrentGrabbleObj (Variables|Default|GetPlayerCharacter))
        (:then
          (Variables|/Game/Blueprints/GrabbleObjects/BP_BaseGrabbleObj.BP_BaseGrabbleObj_C|SetbScaling _currentgrabbleobj true))
        (:else))
      (elif (Utilities|Enum|Equal(Enum) (Variables|Default|GetScaleType) "NewEnumerator1")
        (bind _currentgrabbleobj_2 (Variables|/Game/Blueprints/PlayerCharacter/BP_PlayerCharacter.BP_PlayerCharacter_C|GetCurrentGrabbleObj (Variables|Default|GetPlayerCharacter))
          (:then
            (Variables|/Game/Blueprints/GrabbleObjects/BP_BaseGrabbleObj.BP_BaseGrabbleObj_C|SetbUnscaling _currentgrabbleobj_2 true))
          (:else))))))

(event OnComponentEndOverlap(Box)
  (params (OverlappedComponent :type Primitive%20Component%20Object%20Reference) (OtherActor :type Actor%20Object%20Reference) (OtherComp :type Primitive%20Component%20Object%20Reference) (OtherBodyIndex :type Integer))
  (if (Actor|ActorHasTag OtherActor "GrabbleObject")
    (bind _currentgrabbleobj (Variables|/Game/Blueprints/PlayerCharacter/BP_PlayerCharacter.BP_PlayerCharacter_C|GetCurrentGrabbleObj (Variables|Default|GetPlayerCharacter))
      (:then
        (Variables|/Game/Blueprints/GrabbleObjects/BP_BaseGrabbleObj.BP_BaseGrabbleObj_C|SetbUnscaling _currentgrabbleobj false)
        (Variables|/Game/Blueprints/GrabbleObjects/BP_BaseGrabbleObj.BP_BaseGrabbleObj_C|SetbScaling _currentgrabbleobj false))
      (:else))))

(event EventBeginPlay
  (bind _asbp_player_character (Utilities|Casting|CastToBP_PlayerCharacter (Game|GetPlayerCharacter 0)))
  (Variables|Default|SetPlayerCharacter _asbp_player_character))

(fn ConstructionScript)